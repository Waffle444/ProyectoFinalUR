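; BP_Health is a healing zone that restores the third-person character's health while it stays inside the Box.
; Box overlap begin caches the character and sets Detected, and overlap end clears it.
; A looped Delay adds a fixed amount to VidaActual at short intervals while Detected and below VidaTotal.
; The addition is not clamped, so health can overshoot the maximum.
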(event OnComponentBeginOverlap(Box)
  (params (OverlappedComponent :type Primitive%20Component%20Object%20Reference) (OtherActor :type Actor%20Object%20Reference) (OtherComp :type Primitive%20Component%20Object%20Reference) (OtherBodyIndex :type Integer) (bFromSweep :type Boolean) (SweepResult :type Hit%20Result%20Structure%20%28by%20ref%29))
  (bind _asbp_third_person_character (Utilities|Casting|CastToBP_ThirdPersonCharacter OtherActor))
  (Variables|Default|SetBP%20third%20person%20character _asbp_third_person_character)
  (Variables|Default|Setdetected true)
  (if (and (< (Variables|/Game/ThirdPerson/Blueprints/BP_ThirdPersonCharacter.BP_ThirdPersonCharacter_C|GetVidaActual (Variables|Default|GetBP%20third%20person%20character)) (Variables|/Game/ThirdPerson/Blueprints/BP_ThirdPersonCharacter.BP_ThirdPersonCharacter_C|GetVidaTotal (Variables|Default|GetBP%20third%20person%20character))) (Variables|Default|Getdetected)) :!label _label
    (Variables|/Game/ThirdPerson/Blueprints/BP_ThirdPersonCharacter.BP_ThirdPersonCharacter_C|SetVidaActual (Variables|Default|GetBP%20third%20person%20character) (+ (Variables|/Game/ThirdPerson/Blueprints/BP_ThirdPersonCharacter.BP_ThirdPersonCharacter_C|GetVidaActual (Variables|Default|GetBP%20third%20person%20character)) 2e+01))
    (Utilities|FlowControl|Delay 0.2)
    (goto _label)))

(event OnComponentEndOverlap(Box)
  (params (OverlappedComponent :type Primitive%20Component%20Object%20Reference) (OtherActor :type Actor%20Object%20Reference) (OtherComp :type Primitive%20Component%20Object%20Reference) (OtherBodyIndex :type Integer))
  (Utilities|Casting|CastToBP_ThirdPersonCharacter OtherActor)
  (Variables|Default|Setdetected false))

(event EventBeginPlay)

(event Collision|EventActorBeginOverlap
  (params (OtherActor :type Actor%20Object%20Reference)))

(event EventTick
  (params (DeltaSeconds :type Float%20%28single-precision%29)))

(fn ConstructionScript)